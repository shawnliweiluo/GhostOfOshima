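; Behavior Tree task that finds the current patrol point for an NPC and writes it to the Blackboard as a target location.
; It reads the patrol index from the Blackboard, picks that entry in the NPC's PatrolPath points, and transforms it from path-local to world space.
; It finishes successfully only with a valid path; a failed NPC cast or missing path never calls FinishExecute.
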(event `self.ReceiveExecuteAI`
  (params (OwnerController :type "AIController Object Reference") (ControlledPawn :type "Pawn Object Reference"))
  (bind _asnpc (cast `/Game/Blueprints/NPC/NPC` ControlledPawn))
  (bind _patrolpath (`/Game/Blueprints/NPC/NPC.PatrolPath` _asnpc)
    (:`then`
      (`BTFunctionLibrary.SetBlackboardValueAsVector` (`self.TargetKey`) (`KismetMathLibrary.TransformLocation` (`Actor.GetTransform` _patrolpath) (`|GetArrayItem` (`/Game/Blueprints/NPC/PatrolPath.PathPoints` _patrolpath) (`BTFunctionLibrary.GetBlackboardValueAsInt` (`self.PatrolPathIndexKey`)))))
      (`self.FinishExecute` true))
    (:`else`)))