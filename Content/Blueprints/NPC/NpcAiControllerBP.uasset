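; AI controller for patrolling NPCs that tracks whether the NPC can perceive the player.
; On begin play it runs the NPC behavior tree, caches the controlled NPC and copies the wait time from its patrol path into the blackboard.
; AI perception updates set the CanSeePlayer blackboard key whenever the sensed actor is the player character, reflecting whether sensing succeeded.
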(event `self.ReceiveBeginPlay`
  (`self.RunBehaviorTree` "/Game/Blueprints/NPC/NPC_BehaviorTree.NPC_BehaviorTree")
  (bind _asnpc (cast `/Game/Blueprints/NPC/NPC` (`self.K2_GetPawn`)))
  (bind _output_get (set `self.MyPawn` _asnpc))
  (`BlackboardComponent.SetValueAsFloat` (`AIBlueprintHelperLibrary.GetBlackboard` null) "WaitTime" (`/Game/Blueprints/NPC/PatrolPath.WaitTime` (`/Game/Blueprints/NPC/NPC.PatrolPath` _output_get))))

(event `self.AIPerception.OnTargetPerceptionUpdated`
  (params (Actor :type "Actor Object Reference") (Stimulus :type "AIStimulus Structure"))
  (cast `/Game/Blueprints/Character/PlayerCharacterBP` Actor)
  (`BlackboardComponent.SetValueAsBool` (`AIBlueprintHelperLibrary.GetBlackboard` null) "CanSeePlayer" (`.bSuccessfullySensed` (break `AIStimulus` Stimulus))))

(fn `UserConstructionScript`)